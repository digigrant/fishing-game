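; Quest manager that creates and tracks the game's quantity, size and species quests, each aimed at a target species.
; AddQuest ignores identifiers it already holds, then uses the quest type to pick a data table and looks up the row by identifier.
; The row's fields fill a new type-specific quest object owned by the manager, which is stored in MyQuests and announced through QuestAdded.
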(fn AddQuest
  (params (Type :type E_QuestTypes%20Enum :default "NewEnumerator0") (Identifier :type Name))
  (if (< (Utilities|Array|FindItem (Variables|Default|GetQuestIdentifiers) Identifier) 0)
    (Utilities|Array|Add (Variables|Default|GetQuestIdentifiers) Identifier)
    (switch Utilities|FlowControl|Switch|SwitchonE_QuestTypes Type
      (:NewEnumerator0
        (Development|PrintString 0 "Error: Null Quest Type"))
      (:NewEnumerator3
        (bind _returnvalue (Utilities|GetDataTableRow "/Game/Blueprints/Quests/DT_QuestQuantity.DT_QuestQuantity" Identifier)
          (:then
            (bind _returnvalue_2 (Game|ConstructObjectfromClass "/Game/Blueprints/Quests/BP_QuestQuantity.BP_QuestQuantity_C" self (.TargetAmount (Utilities|Struct|BreakF_QuestQuantity _returnvalue)) (.TargetSpecies (Utilities|Struct|BreakF_QuestQuantity _returnvalue)) (.QuestName (Utilities|Struct|BreakF_QuestQuantity _returnvalue)) (.QuestDescription (Utilities|Struct|BreakF_QuestQuantity _returnvalue))))
            (Utilities|Array|Add (Variables|Default|GetMyQuests) _returnvalue_2)
            (Default|CallQuestAdded _returnvalue_2))))
      (:NewEnumerator1
        (bind _returnvalue_3 (Utilities|GetDataTableRow "/Game/Blueprints/Quests/DT_QuestSize.DT_QuestSize" Identifier)
          (:then
            (bind _returnvalue_4 (Game|ConstructObjectfromClass "/Game/Blueprints/Quests/BP_QuestSize.BP_QuestSize_C" self (.TargetSpecies (Utilities|Struct|BreakF_QuestSize _returnvalue_3)) (.TargetSize (Utilities|Struct|BreakF_QuestSize _returnvalue_3)) (.QuestName (Utilities|Struct|BreakF_QuestSize _returnvalue_3)) (.QuestDescription (Utilities|Struct|BreakF_QuestSize _returnvalue_3))))
            (Utilities|Array|Add (Variables|Default|GetMyQuests) _returnvalue_4)
            (Default|CallQuestAdded _returnvalue_4))))
      (:NewEnumerator2
        (bind _returnvalue_5 (Utilities|GetDataTableRow "/Game/Blueprints/Quests/DT_QuestSpecies.DT_QuestSpecies" Identifier)
          (:then
            (bind _returnvalue_6 (Game|ConstructObjectfromClass "/Game/Blueprints/Quests/BP_QuestSpecies.BP_QuestSpecies_C" self (.TargetSpecies (Utilities|Struct|BreakF_QuestSpecies _returnvalue_5)) (.QuestName (Utilities|Struct|BreakF_QuestSpecies _returnvalue_5)) (.QuestDescription (Utilities|Struct|BreakF_QuestSpecies _returnvalue_5))))
            (Utilities|Array|Add (Variables|Default|GetMyQuests) _returnvalue_6)
            (Default|CallQuestAdded _returnvalue_6)))))))
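; Game instance for a fishing game that holds player state across levels: inventory, quests and money.
; On Init it constructs an inventory object seeded with starter bait, a rod and a lure, then constructs a quest manager.
; AddMoney ignores non-positive amounts, and DeductMoney clamps the balance at zero.
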(event EventInit
  (bind _returnvalue (Game|ConstructObjectfromClass "/Game/Blueprints/Inventory/BP_Inventory.BP_Inventory_C" self))
  (bind _output_get (Variables|Default|SetMyInventory _returnvalue))
  (Default|AddBait _output_get (Utilities|Struct|MakeF_BaitInstance "Worm" 10))
  (Default|AddRod _output_get "OkayRod")
  (Default|AddLure _output_get "Jig")
  (bind _returnvalue_2 (Game|ConstructObjectfromClass "/Game/Blueprints/Quests/BP_QuestManager.BP_QuestManager_C" self))
  (Variables|Default|SetMyQuestManager _returnvalue_2))

(fn AddMoney
  (params (NewMoney :type Float%20%28single-precision%29))
  (if (> NewMoney 0.0)
    (Variables|Default|SetCurrentMoney (+ NewMoney (Variables|Default|GetCurrentMoney)))))

(fn DeductMoney
  (params (Amount :type Float%20%28single-precision%29))
  (Variables|Default|SetCurrentMoney (Math|Float|Max(Float) (- (Variables|Default|GetCurrentMoney) Amount) 0.0)))
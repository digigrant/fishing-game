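; BP_ShopInventory is the shop's inventory of fishing gear, stocked from the rod, bait and lure data tables.
; InitShop walks every row name in each table, adding rods and lures by name alone.
; Bait rows are looked up so each is added as a bait instance carrying the row's Quantity as its amount.
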(fn InitShop
  (bind _outrownames (DataTable|GetDataTableRowNames "/Game/Blueprints/Inventory/DT_Rods.DT_Rods"))
  (for _array_element _outrownames
    (CallFunction|AddRod _array_element))
  (bind _outrownames_2 (DataTable|GetDataTableRowNames "/Game/Blueprints/Inventory/DT_Bait.DT_Bait"))
  (for _array_element_2 _outrownames_2
    (bind _returnvalue (Utilities|GetDataTableRow "/Game/Blueprints/Inventory/DT_Bait.DT_Bait" _array_element_2)
      (:then
        (CallFunction|AddBait (Utilities|Struct|MakeF_BaitInstance _array_element_2 (.Quantity (Utilities|Struct|BreakF_Bait _returnvalue)))))))
  (bind _outrownames_3 (DataTable|GetDataTableRowNames "/Game/Blueprints/Inventory/DT_Lures.DT_Lures"))
  (for _array_element_3 _outrownames_3
    (CallFunction|AddLure _array_element_3)))
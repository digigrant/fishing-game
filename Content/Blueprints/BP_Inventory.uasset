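; BP_Inventory stores the fishing gear and catch in a fishing game: bait, rods, lures and caught fish.
; Add functions validate bait, rods and lures against their DataTables, while fish are appended directly.
; Bait stacks by identifier with an amount, and the other items are individual array entries.
; CurrentCapacity counts occupied entries as they are added or removed, with no limit checked here.
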(fn AddBait
  (params (NewBait :type F%20Bait%20Instance%20Structure))
  (bind (_identifier _amount) (Utilities|Struct|BreakF_BaitInstance NewBait))
  (Utilities|GetDataTableRow "/Game/GameData/Items/DT_Bait.DT_Bait" _identifier
    (:then
      (for (_array_element _array_index) (Variables|Default|GetBait)
        (if (Utilities|Name|Equal(Name) (.Identifier (Utilities|Struct|BreakF_BaitInstance _array_element)) _identifier)
          (Utilities|Struct|SetmembersinF_BaitInstance (Utilities|Array|Get(acopy) (Variables|Default|GetBait) _array_index) (+ (.Amount (Utilities|Struct|BreakF_BaitInstance (Utilities|Array|Get(acopy) (Variables|Default|GetBait) _array_index))) _amount))
          (return)))
      (Utilities|Array|Add (Variables|Default|GetBait) NewBait)
      (Math|Integer|IncrementInt (Variables|Default|GetCurrentCapacity)))))

(fn AddRod
  (params (RodName :type Name))
  (Utilities|GetDataTableRow "/Game/GameData/Items/DT_Rods.DT_Rods" RodName
    (:then
      (Utilities|Array|Add (Variables|Default|GetRods) RodName)
      (Math|Integer|IncrementInt (Variables|Default|GetCurrentCapacity)))
    (:RowNotFound
      (Development|PrintString 0 "Error: Rod not found"))))

(fn AddLure
  (params (NewLure :type Name))
  (Utilities|GetDataTableRow "/Game/GameData/Items/DT_Lures.DT_Lures" NewLure
    (:then
      (Utilities|Array|Add (Variables|Default|GetLures) NewLure)
      (Math|Integer|IncrementInt (Variables|Default|GetCurrentCapacity)))
    (:RowNotFound
      (Development|PrintString 0 "Error: Lure not found"))))

(fn AddFish
  (params (NewFish :type F%20Caught%20Fish%20Structure))
  (Utilities|Array|Add (Variables|Default|GetCaughtFish) NewFish)
  (Math|Integer|IncrementInt (Variables|Default|GetCurrentCapacity)))

(fn RemoveBait
  (params (Bait :type F%20Bait%20Instance%20Structure))
  (bind (_identifier _amount) (Utilities|Struct|BreakF_BaitInstance Bait))
  (for (_array_element _array_index) (Variables|Default|GetBait)
    (if (Utilities|Name|Equal(Name) (.Identifier (Utilities|Struct|BreakF_BaitInstance _array_element)) _identifier)
      (if (> (- (.Amount (Utilities|Struct|BreakF_BaitInstance _array_element)) _amount) 0)
        (Utilities|Struct|SetmembersinF_BaitInstance _array_element (- (.Amount (Utilities|Struct|BreakF_BaitInstance _array_element)) _amount))
        (else
          (Utilities|Array|RemoveIndex (Variables|Default|GetBait) _array_index)
          (Math|Integer|DecrementInt (Variables|Default|GetCurrentCapacity)
            (:%20%20
              _))))
      (return))))

(fn RemoveRod
  (params (Identifier :type Name))
  (bind _returnvalue (Utilities|Array|RemoveItem (Variables|Default|GetRods) Identifier))
  (if _returnvalue
    (Math|Integer|DecrementInt (Variables|Default|GetCurrentCapacity))))

(fn RemoveLure
  (params (Identifier :type Name))
  (bind _returnvalue (Utilities|Array|RemoveItem (Variables|Default|GetLures) Identifier))
  (if _returnvalue
    (Math|Integer|DecrementInt (Variables|Default|GetCurrentCapacity))))

(fn RemoveFish
  (params (Index :type Integer))
  (Utilities|Array|RemoveIndex (Variables|Default|GetCaughtFish) Index)
  (Math|Integer|DecrementInt (Variables|Default|GetCurrentCapacity)))
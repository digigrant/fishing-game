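; Blueprint function library with small HUD and text helpers.
; GetPlayerHUDWidget casts a player controller's HUD to BP_FirstPersonHUD and returns its MyWidget.
; FormatFloat turns a float into a string, splits it at the decimal point and keeps the requested number of decimal characters, truncating rather than rounding.
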(fn GetPlayerHUDWidget
  (params (PlayerController :type Player%20Controller%20Object%20Reference))
  (bind _asbp_first_person_hud (Utilities|Casting|CastToBP_FirstPersonHUD (HUD|GetHUD PlayerController)))
  (return (Variables|/Game/Blueprints/UI/BP_FirstPersonHUD.BP_FirstPersonHUD_C|GetMyWidget _asbp_first_person_hud)))

(fn FormatFloat
  (params (Float :type Float%20%28single-precision%29) (Precision :type Integer))
  (bind _returnvalue (Utilities|String|ToString(Float) Float))
  (bind _returnvalue_2 (Utilities|String|ParseIntoArray _returnvalue "."))
  (return (Utilities|String|Append (Utilities|Array|Get(acopy) _returnvalue_2) "." (Utilities|String|GetSubstring (Utilities|Array|Get(acopy) _returnvalue_2 1) 0 Precision))))
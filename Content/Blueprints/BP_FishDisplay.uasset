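; BP_FishDisplay is a fish display that shows its skeletal mesh according to that species' entry in the player's Fishdex.
; On BeginPlay it searches the SpeciesSkeletalMesh column of DT_FishSpecies for its own mesh, comparing the asset name cut from each path string.
; The matching row index reads the Fishdex boolean in BP_FishingGameInstance to set mesh visibility, so both must share the same order.
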(event EventBeginPlay
  (bind _returnvalue (Class|DataTableFunctionLibrary|GetDataTableColumnasString "/Game/GameData/Fish/FishSpecies/DT_FishSpecies.DT_FishSpecies" "SpeciesSkeletalMesh"))
  (bind (_array_element _array_index) (Utilities|Array|ForEachLoopwithBreak _returnvalue :!label _label)
    (:LoopBody
      (if (Utilities|Enum|Equal(Enum) (Utilities|String|ToString(Object) (Variables|/Script/Engine.SkinnedMeshComponent|GetSkeletalMesh (Variables|Default|GetMySkeletalMesh))) (Utilities|String|GetSubstring _array_element (+ (Utilities|Array|FindItem (Utilities|String|GetCharacterArrayfromString _array_element) ".") 1) (- (- (Utilities|String|Len _array_element) (Utilities|Array|FindItem (Utilities|String|GetCharacterArrayfromString _array_element) ".")) 2)))
        (bind _asbp_fishing_game_instance (Utilities|Casting|CastToBP_FishingGameInstance (Game|GetGameInstance)))
        (Rendering|SetVisibility (Variables|Default|GetMySkeletalMesh) (Utilities|Array|Get(acopy) (Variables|/Game/Blueprints/BP_FishingGameInstance.BP_FishingGameInstance_C|GetFishdex _asbp_fishing_game_instance) _array_index) false)
        (goto _label Break)))))

(fn ConstructionScript)
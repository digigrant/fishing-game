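; Game instance for the fishing game, holding persistent state: inventory with starter gear, money, quests, tutorial flags, Fishdex and pond access.
; Caught fish go to the inventory and update every quest; completed quests advance that quest type's next NPC dialogue.
; Character look and move events complete tutorial flags once, then unbind.
; Level changes run through a loading widget, opening the level after fade-in, then fading out.
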(event Custom|OnLook
  (EventDispatchers|UnbindEventfromOnLook (stale Custom|OnCharacterInitComplete _asbpc_cabin_character) (delegate Custom|OnLook))
  (CallFunction|SetTutorialFlagtoComplete "NewEnumerator0"))

(event Custom|OnQuestUpdated
  (params (Quest :type BP%20Quest%20Object%20Reference))
  (bind _questtype (Variables|/Game/Blueprints/Quests/BP_Quest.BP_Quest_C|GetQuestType Quest))
  (bind _returnvalue (Math|Conversions|ToInteger(Byte) _questtype))
  (if (Variables|/Game/Blueprints/Quests/BP_Quest.BP_Quest_C|GetIsComplete Quest)
    (CallFunction|SetNextNPCDialogue _returnvalue (+ (Utilities|Array|Get(acopy) (Variables|Default|GetNextNPCDialogue) _returnvalue) 1))))

(event Custom|OnMove
  (EventDispatchers|UnbindEventfromOnMove (stale Custom|OnCharacterInitComplete _asbpc_cabin_character) (delegate Custom|OnMove))
  (CallFunction|SetTutorialFlagtoComplete "NewEnumerator1"))

(event Custom|OnCharacterInitComplete
  (params (Character :type Character%20Object%20Reference))
  (bind _asbpc_cabin_character (Utilities|Casting|CastToBPC_CabinCharacter Character))
  (EventDispatchers|BindEventtoOnLook _asbpc_cabin_character (delegate Custom|OnLook))
  (EventDispatchers|BindEventtoOnMove _asbpc_cabin_character (delegate Custom|OnMove)))

(event Custom|OnLoadingFadeIn_Complete
  (bind _transitionwidget (Variables|Default|GetTransitionWidget))
  (Game|OpenLevel(byName) (Variables|Default|GetLevelToLoad))
  (UserInterface|Animation|PlayAnimation _transitionwidget (Variables|/Game/Blueprints/UI/BPUI_Loading.BPUI_Loading_C|GetFadeOut _transitionwidget) 0.0 1 "Forward" 1.0))

(event Custom|OnLoadingFadeOutComplete
  (Widget|RemovefromParent (Variables|Default|GetTransitionWidget))
  (Input|SetInputModeGameOnly (Game|GetPlayerController 0)))

(event EventInit
  (bind _pondaccess (Variables|Default|GetPondAccess))
  (bind _returnvalue (Game|ConstructObjectfromClass "/Game/Blueprints/BP_Inventory.BP_Inventory_C" self))
  (bind _output_get (Variables|Default|SetMyInventory _returnvalue))
  (Default|AddBait _output_get (Utilities|Struct|MakeF_BaitInstance "Worm" 10))
  (Default|AddRod _output_get "OkayRod")
  (Default|AddLure _output_get "Jig")
  (bind _returnvalue_2 (Game|ConstructObjectfromClass "/Game/Blueprints/Quests/BP_QuestManager.BP_QuestManager_C" self))
  (bind _output_get_2 (Variables|Default|SetMyQuestManager _returnvalue_2))
  (EventDispatchers|BindEventtoQuestUpdated _output_get_2 (delegate Custom|OnQuestUpdated))
  (Default|InitializeQuestManager _output_get_2)
  (Utilities|Array|Resize (Variables|Default|GetTutorialFlags) (|GetNumEnumEntries))
  (Utilities|Array|Resize (Variables|Default|GetNextNPCDialogue) 4)
  (CallFunction|ResetFishdex)
  (Utilities|Array|Resize _pondaccess 3)
  (Utilities|Array|SetArrayElem _pondaccess 0 true)
  (bind _returnvalue_3 (UserInterface|CreateWidget "/Game/Blueprints/UI/BPUI_Loading.BPUI_Loading_C" (Game|GetPlayerController 0)))
  (bind _output_get_3 (Variables|Default|SetTransitionWidget _returnvalue_3))
  (EventDispatchers|BindEventtoOnAnimationFinished (Variables|/Game/Blueprints/UI/BPUI_Loading.BPUI_Loading_C|GetFadeIn _output_get_3) (delegate Custom|OnLoadingFadeIn_Complete))
  (EventDispatchers|BindEventtoOnAnimationFinished (Variables|/Game/Blueprints/UI/BPUI_Loading.BPUI_Loading_C|GetFadeOut _output_get_3) (delegate Custom|OnLoadingFadeOutComplete)))

(fn AddMoney
  (params (NewMoney :type Float%20%28single-precision%29))
  (if (> NewMoney 0.0)
    (Variables|Default|SetCurrentMoney (+ NewMoney (Variables|Default|GetCurrentMoney)))))

(fn DeductMoney
  (params (Amount :type Float%20%28single-precision%29))
  (Variables|Default|SetCurrentMoney (Math|Float|Max(Float) (- (Variables|Default|GetCurrentMoney) Amount) 0.0)))

(fn SetTutorialFlagtoComplete
  (params (Tutorial :type E_Tutorials%20Enum :default "NewEnumerator2"))
  (Utilities|Array|SetArrayElem (Variables|Default|GetTutorialFlags) (Math|Conversions|ToInteger(Byte) Tutorial) true))

(fn GetTutorialFlag
  (params (Tutorial :type E_Tutorials%20Enum :default "NewEnumerator2"))
  (return (Utilities|Array|Get(acopy) (Variables|Default|GetTutorialFlags) (Math|Conversions|ToInteger(Byte) Tutorial))))

(fn SetNextNPCDialogue
  (params (NPC_ID :type Integer) (Conversation_ID :type Integer))
  (Utilities|Array|SetArrayElem (Variables|Default|GetNextNPCDialogue) NPC_ID Conversation_ID))

(fn AddFishtoInventory
  (params (NewFish :type F%20Caught%20Fish%20Structure))
  (Default|AddFish (Variables|Default|GetMyInventory) NewFish)
  (for _array_element (Variables|/Game/Blueprints/Quests/BP_QuestManager.BP_QuestManager_C|GetMyQuests (Variables|Default|GetMyQuestManager))
    (Default|UpdateQuest _array_element NewFish)))

(fn ResetFishdex
  (Utilities|Array|Clear (Variables|Default|GetFishdex))
  (bind _outrownames (DataTable|GetDataTableRowNames "/Game/GameData/Fish/FishSpecies/DT_FishSpecies.DT_FishSpecies"))
  (Utilities|Array|Resize (Variables|Default|GetFishdex) (Utilities|Array|Length _outrownames)))

(fn AddtoFishdex
  (params (FishName :type Name))
  (bind _outrownames (DataTable|GetDataTableRowNames "/Game/GameData/Fish/FishSpecies/DT_FishSpecies.DT_FishSpecies"))
  (Utilities|Array|SetArrayElem (Variables|Default|GetFishdex) (Utilities|Array|FindItem _outrownames FishName) true))

(fn TransitiontoNewLevel
  (params (NewLevel :type Name))
  (bind _transitionwidget (Variables|Default|GetTransitionWidget))
  (Variables|Default|SetLevelToLoad NewLevel)
  (Input|SetInputModeUIOnly (Game|GetPlayerController 0) _transitionwidget "DoNotLock")
  (UserInterface|Viewport|AddtoViewport _transitionwidget 0)
  (UserInterface|Animation|PlayAnimation _transitionwidget (Variables|/Game/Blueprints/UI/BPUI_Loading.BPUI_Loading_C|GetFadeIn _transitionwidget) 0.0 1 "Forward" 1.0))
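; Quest blueprint that tracks catching a target quantity of a specific fish species.
; UpdateQuest compares the passed fish's species name to the target and increments the progress count on a match.
; When the count reaches the target amount, it marks the quest complete and calls the quest-complete dispatch.
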(event EventUpdateQuest
  (params (Fish :type F%20Caught%20Fish%20Structure))
  (if (Utilities|Name|Equal(Name) (.SpeciesName (Utilities|Struct|BreakF_CaughtFish Fish)) (Variables|Default|GetTargetSpecies))
    (Math|Integer|IncrementInt (Variables|Default|GetCurrent)
      (:%20%20
        (if (not (< (Variables|Default|GetCurrent) (Variables|Default|GetTargetAmount)))
          (Variables|Default|SetIsComplete true)
          (Default|CallQuestComplete))))))
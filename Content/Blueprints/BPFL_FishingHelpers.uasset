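; Blueprint function library for fishing, with an EvaluateFish function that computes a value for a caught fish.
; It chains data table lookups: species name gives the rarity, then the rarity and weight category enums become row names in their own tables.
; The result is the rarity's base value times its root value raised to the weight's modifier, so weight scales value exponentially.
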(fn EvaluateFish
  (params (CaughtFish :type F%20Caught%20Fish%20Structure))
  (bind (_speciesname _weightcategory) (Utilities|Struct|BreakF_CaughtFish CaughtFish))
  (bind _returnvalue (Utilities|GetDataTableRow "/Game/GameData/Fish/FishSpecies/DT_FishSpecies.DT_FishSpecies" _speciesname)
    (:then
      (bind _returnvalue_2 (Utilities|GetDataTableRow "/Game/GameData/Fish/FishSpecies/DT_Rarity.DT_Rarity" (Utilities|String|StringToName (Utilities|String|EnumtoString (.SpeciesRarity (Utilities|Struct|BreakF_FishSpecies _returnvalue)))))
        (:then
          (bind _returnvalue_3 (Utilities|GetDataTableRow "/Game/GameData/Fish/FishSpecies/DT_Weight.DT_Weight" (Utilities|String|StringToName (Utilities|String|EnumtoString _weightcategory)))
            (:then
              (return (* (Math|Float|Power (.RootValue (Utilities|Struct|BreakF_FishRarity _returnvalue_2)) (.ValueModifer (Utilities|Struct|BreakF_FishWeight _returnvalue_3))) (.BaseValue (Utilities|Struct|BreakF_FishRarity _returnvalue_2)))))))))))
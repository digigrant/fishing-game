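; BP_Bobber is a fishing bobber projectile that floats in pond volumes and runs the bite-and-catch state machine.
; Pond overlaps toggle gravity, with drag and upward force faking buoyancy, and start the WAIT state.
; A timer advances WAIT to ALERT, then REHOOK, while driving a reeling icon widget.
; Reeling during ALERT spawns a fish chosen by the pond and attaches it to the hook.
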(event OnComponentBeginOverlap(Collider)
  (params (OverlappedComponent :type Primitive%20Component%20Object%20Reference) (OtherActor :type Actor%20Object%20Reference) (OtherComp :type Primitive%20Component%20Object%20Reference) (OtherBodyIndex :type Integer) (bFromSweep :type Boolean) (SweepResult :type Hit%20Result%20Structure%20%28by%20ref%29))
  (bind _collider (Variables|Default|GetCollider))
  (bind _returnvalue (Transformation|GetComponentVelocity _collider))
  ;[1 1 1] Physics
  (Utilities|Casting|CastToBP_PondVolume OtherActor)
  (Physics|SetEnableGravity _collider false)
  (Physics|SetPhysicsLinearVelocity _collider (Math|Vector|MakeVector (.x _returnvalue) (.y _returnvalue) (* (.z _returnvalue) 0.1)) false "None"))

(event OnComponentEndOverlap(Collider)
  (params (OverlappedComponent :type Primitive%20Component%20Object%20Reference) (OtherActor :type Actor%20Object%20Reference) (OtherComp :type Primitive%20Component%20Object%20Reference) (OtherBodyIndex :type Integer))
  ;[1 1 1] Physics
  (Utilities|Casting|CastToBP_PondVolume OtherActor)
  (Physics|SetEnableGravity (Variables|Default|GetCollider) true))

(event OnComponentBeginOverlap(PondCollider)
  (params (OverlappedComponent :type Primitive%20Component%20Object%20Reference) (OtherActor :type Actor%20Object%20Reference) (OtherComp :type Primitive%20Component%20Object%20Reference) (OtherBodyIndex :type Integer) (bFromSweep :type Boolean) (SweepResult :type Hit%20Result%20Structure%20%28by%20ref%29))
  ;[1 1 1] Pond Detection
  (bind _asbp_pond_volume (Utilities|Casting|CastToBP_PondVolume OtherActor))
  (Variables|Default|SetCurrentPond _asbp_pond_volume)
  (CallFunction|SetNewBobberState "NewEnumerator1"))

(event OnComponentEndOverlap(PondCollider)
  (params (OverlappedComponent :type Primitive%20Component%20Object%20Reference) (OtherActor :type Actor%20Object%20Reference) (OtherComp :type Primitive%20Component%20Object%20Reference) (OtherBodyIndex :type Integer))
  ;[1 1 1] Pond Detection
  (Utilities|Casting|CastToBP_PondVolume OtherActor)
  (Variables|Default|SetCurrentPond 0)
  (CallFunction|SetNewBobberState "NewEnumerator0"))

(event Custom|OnReel
  (params (IsReeling :type Boolean))
  (switch Utilities|FlowControl|Switch|SwitchonE_BobberIconStates (Variables|Default|GetCurrentState)
    (:NewEnumerator2
      (CallFunction|CatchFishfromCurrentPond)
      (CallFunction|SetNewBobberState "NewEnumerator4"))))

(event EventBeginPlay
  (bind _asbpw_reeling_icon (Utilities|Casting|CastToBPW_ReelingIcon (UserInterface|GetUserWidgetObject (Variables|Default|GetWidget))))
  (Variables|Default|SetMyReelingIcon _asbpw_reeling_icon)
  (CallFunction|SetNewBobberState "NewEnumerator0"))

(event EventTick
  (params (DeltaSeconds :type Float%20%28single-precision%29))
  (CallFunction|UpdateBobber DeltaSeconds))

(fn ConstructionScript
  (bind _projectilemovement (Variables|Default|GetProjectileMovement))
  (Variables|/Script/Engine.ProjectileMovementComponent|SetInitialSpeed _projectilemovement (* (Class|MovementComponent|GetMaxSpeed _projectilemovement) (Variables|Default|GetProjectileSpeed))))

(fn CatchFishfromCurrentPond
  (bind _self self)
  (Utilities|IsValid (Variables|Default|GetCurrentPond)
    (:Is%20Valid
      (Utilities|IsValid (Variables|Default|GetMyCaughtFish)
        (:Is%20Not%20Valid
          (bind _fish (Default|ChooseFish (Variables|Default|GetCurrentPond)))
          (bind _returnvalue (Game|SpawnActorfromClass "/Game/Blueprints/BP_Fish.BP_Fish_C" (Math|Transform|MakeTransform (Transformation|GetActorLocation _self) (Transformation|GetActorRotation _self)) "Undefined" _self _fish 0))
          (bind _output_get (Variables|Default|SetMyCaughtFish _returnvalue))
          (Transformation|AttachComponentToComponent (Variables|/Game/Blueprints/BP_Fish.BP_Fish_C|GetChomper _output_get) (Variables|Default|GetHook) "None" "SnapToTarget" "SnapToTarget" "KeepWorld" false))))))

(fn ReleaseFish
  (bind _mycaughtfish (Variables|Default|GetMyCaughtFish))
  (Utilities|IsValid _mycaughtfish
    (:Is%20Valid
      (Actor|DestroyActor _mycaughtfish))))

(fn UpdateBobber
  (params (DeltaTime :type Float%20%28single-precision%29))
  (bind _collider (Variables|Default|GetCollider))
  (bind _collider_2 (Variables|Default|GetCollider))
  (bind _returnvalue (Transformation|GetComponentVelocity _collider))
  (Utilities|FlowControl|Sequence
    (:then_0
      (if (not (Class|PrimitiveComponent|IsGravityEnabled (Variables|Default|GetCollider)))
        (Physics|AddForce _collider_2 (* (Math|Vector|MakeVector (.x _returnvalue) (.y _returnvalue) 0.0) (* DeltaTime (Math|Float|MakeLiteralFloat -4e+02))) "None" true)
        (Physics|AddForce _collider_2 "0, 0,500.000000" "None" true)))
    (:then_1
      (if (> (Variables|Default|GetTimer) 0.0)
        (bind _output_get (Variables|Default|SetTimer (- (Variables|Default|GetTimer) DeltaTime)))
        (Utilities|FlowControl|Sequence
          (:then_0
            (if (Utilities|Enum|Equal(Enum) (Variables|Default|GetCurrentState) "NewEnumerator2")
              (Default|UpdateIconFillPercent (Variables|Default|GetMyReelingIcon) (- 1.0 (/ (Variables|Default|GetTimer) (Math|Float|MakeLiteralFloat 3.0))))))
          (:then_1
            (if (< _output_get 0.0)
              (switch Utilities|FlowControl|Switch|SwitchonE_BobberIconStates (Variables|Default|GetCurrentState)
                (:NewEnumerator1
                  (CallFunction|SetNewBobberState "NewEnumerator2"))
                (:NewEnumerator2
                  (CallFunction|SetNewBobberState "NewEnumerator3"))))))))))

(fn SetNewBobberState
  (params (NewState :type E_BobberIconStates%20Enum :default "NewEnumerator0"))
  (Default|SetState (Variables|Default|GetMyReelingIcon) NewState)
  (Variables|Default|SetCurrentState NewState)
  (switch Utilities|FlowControl|Switch|SwitchonE_BobberIconStates NewState
    (:NewEnumerator1
      (Variables|Default|SetTimer 3.0))
    (:NewEnumerator2
      (Variables|Default|SetTimer 3.0))))